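; BP_PhantomObj is an interactable object that temporarily vanishes when its Interaction event is triggered with a projectile.
; The event destroys the projectile, then hides the mesh and switches its collision profile to NoCollision.
; A timeline serves as the delay, and when it finishes the mesh becomes visible again and blocks all dynamic objects.
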(event EventBeginPlay)

(event Collision|EventActorBeginOverlap
  (params (OtherActor :type Actor%20Object%20Reference)))

(event EventTick
  (params (DeltaSeconds :type Float%20%28single-precision%29)))

(event EventInteraction
  (params (Projectile :type Actor%20Object%20Reference))
  (Actor|DestroyActor Projectile)
  (Rendering|SetVisibility (Variables|Character|GetMesh) false false)
  (Collision|SetCollisionProfileName (Variables|Character|GetMesh) "NoCollision" true :!class /Script/Engine.PrimitiveComponent)
  (Timeline|타임라인_0 PlayFromStart
    (:Finished
      (Rendering|SetVisibility (Variables|Character|GetMesh) true false)
      (Collision|SetCollisionProfileName (Variables|Character|GetMesh) "BlockAllDynamic" true :!class /Script/Engine.PrimitiveComponent))))

(fn ConstructionScript)