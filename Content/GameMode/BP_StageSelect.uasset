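; BP_StageSelect is an actor that sends the player to a stage level on contact.
; When its StaticMesh is hit by a SideScrollerCharacter, it calls IsStage on the PortalEXGameInstance and prints a debug "Hello".
; It then saves its MStageData through the game instance, loads it back and opens the level named in that data.
; BeginPlay, overlap and Tick are unused.
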(event OnComponentHit(StaticMesh)
  (params (HitComponent :type Primitive%20Component%20Object%20Reference) (OtherActor :type Actor%20Object%20Reference) (OtherComp :type Primitive%20Component%20Object%20Reference) (NormalImpulse :type Vector :default "0, 0, 0") (Hit :type Hit%20Result%20Structure%20%28by%20ref%29))
  (Utilities|Casting|CastToSideScrollerCharacter OtherActor)
  (bind _asportal_exgame_instance (Utilities|Casting|CastToPortalEXGameInstance (Game|GetGameInstance)))
  (Class|PortalEXGameInstance|IsStage _asportal_exgame_instance)
  (Development|PrintString "Hello")
  (Class|PortalEXGameInstance|Save _asportal_exgame_instance (Variables|Default|GetmStageData))
  (bind _returnvalue (Class|PortalEXGameInstance|Load _asportal_exgame_instance (Variables|Default|GetmStageData)))
  (Variables|Default|SetmStageData _returnvalue)
  (Game|OpenLevel(byName) (Utilities|String|StringToName (.levelname (Variables|Default|GetmStageData)))))

(event EventBeginPlay)

(event Collision|EventActorBeginOverlap
  (params (OtherActor :type Actor%20Object%20Reference)))

(event EventTick
  (params (DeltaSeconds :type Float%20%28single-precision%29)))

(fn ConstructionScript)