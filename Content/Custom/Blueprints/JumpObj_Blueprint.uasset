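; JumpObj_Blueprint is an actor that restarts the game when it detects the side-scroller character.
; An overlap on its Box component triggers a multi box trace for objects, centered just below the actor.
; Each hit that casts to TP_SideScrollerCharacter calls Restart on BP_PortalEXGameState.
; Debug prints and trace drawing are left on.
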(event OnComponentBeginOverlap(Box)
  (params (OverlappedComponent :type Primitive%20Component%20Object%20Reference) (OtherActor :type Actor%20Object%20Reference) (OtherComp :type Primitive%20Component%20Object%20Reference) (OtherBodyIndex :type Integer) (bFromSweep :type Boolean) (SweepResult :type Hit%20Result%20Structure%20%28by%20ref%29))
  (bind _returnvalue (Transformation|GetActorLocation))
  (bind _returnvalue_2 (+ _returnvalue "0, 0,-50.000000"))
  (Development|PrintString "Hello")
  (bind _outhits (Class|KismetSystemLibrary|BoxTraceMultiforObjects _returnvalue_2 _returnvalue_2 "70.000000,70.000000,70.000000" "0, 0, 0" (Variables|Default|GetObject%20Types) false 0 "ForDuration" true))
  (for _array_element _outhits
    (Utilities|Casting|CastToTP_SideScrollerCharacter (.HitActor (Collision|BreakHitResult _array_element)))
    (Development|PrintString "Restart")
    (bind _asbp_portal_exgame_state (Utilities|Casting|CastToBP_PortalEXGameState (Game|GetGameState)))
    (Class|PortalEXGameStateBase|Restart _asbp_portal_exgame_state)))

(event EventBeginPlay)

(event Collision|EventActorBeginOverlap
  (params (OtherActor :type Actor%20Object%20Reference)))

(event EventTick
  (params (DeltaSeconds :type Float%20%28single-precision%29)))

(fn ConstructionScript)