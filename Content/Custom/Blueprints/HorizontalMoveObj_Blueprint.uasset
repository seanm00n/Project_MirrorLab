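; Blueprint for a horizontally moving object, with a Mesh and Left and Right points used as trace origins.
; IsMovable line-traces along world Y from Right toward -Y for positive Dir, otherwise from Left toward +Y, over the given distance.
; It returns true when the trace hits something, with debug print and drawing left on.
; Event handlers are empty, and the move, destroy and interaction nodes are disconnected, so nothing here moves the object.
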(event EventBeginPlay)

(event Collision|EventActorBeginOverlap
  (params (OtherActor :type Actor%20Object%20Reference)))

(event EventTick
  (params (DeltaSeconds :type Float%20%28single-precision%29)))

(fn ConstructionScript)

(fn IsMovable
  (params (dir :type Float%20%28single-precision%29) (distance :type Float%20%28single-precision%29))
  (bind _left (Variables|Default|GetLeft))
  (bind _right (Variables|Default|GetRight))
  (bind _returnvalue (Transformation|GetWorldLocation _left))
  (bind _returnvalue_2 (Transformation|GetWorldLocation _right))
  (Development|PrintString "trace")
  (LocalVariables|SetLocalDistance distance)
  (LocalVariables|SetLocalDir dir)
  (if (> (LocalVariables|GetLocalDir) 0.0)
    (bind _returnvalue_3 (Class|KismetSystemLibrary|LineTraceMultiforObjects (Transformation|GetWorldLocation _right) (Math|Vector|MakeVector (.x _returnvalue_2) (- (.y _returnvalue_2) (LocalVariables|GetLocalDistance)) (.z _returnvalue_2)) (LocalVariables|GetTraceTypes) false 0 "ForDuration" true))
    (if _returnvalue_3
      _
      (else
        (return false)))
    (else
      (bind _returnvalue_4 (Class|KismetSystemLibrary|LineTraceMultiforObjects (Transformation|GetWorldLocation _left) (Math|Vector|MakeVector (.x _returnvalue) (+ (.y _returnvalue) (LocalVariables|GetLocalDistance)) (.z _returnvalue)) (LocalVariables|GetTraceTypes) false 0 "ForDuration" true))
      (if _returnvalue_4
        _
        (else
          (return false)))))
  (return true))